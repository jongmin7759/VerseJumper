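; Main menu double door actor that plays a continuously repeating opening animation as backdrop motion.
; The construction script caches both panels' initial relative locations.
; From BeginPlay, a timeline slides the left and right panels in opposite directions along local X, scaled by an open distance.
; When the timeline finishes, OpenDoor calls itself to replay from the start, looping indefinitely.
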(event Custom|OpenDoor
  (bind _alpha (Timeline|DoorMovement PlayFromStart)
    (:Update
      (bind _output_get (Variables|Default|SetAlpha _alpha))
      (Transformation|SetRelativeLocation (Variables|Default|GetDoor_L) (+ (Variables|Default|GetInitialLoc_L) (Math|Vector|MakeVector (* _output_get (Variables|Default|GetOpenDist) -1.0) 0.0 0.0)) false false)
      (Transformation|SetRelativeLocation (Variables|Default|GetDoor_R) (+ (Variables|Default|GetInitialLoc_R) (Math|Vector|MakeVector (* (Variables|Default|GetAlpha) (Variables|Default|GetOpenDist)) 0.0 0.0)) false false))
    (:Finished
      (CallFunction|OpenDoor))))

(event EventBeginPlay
  (CallFunction|OpenDoor))

(fn ConstructionScript
  (Variables|Default|SetInitialLoc_L (Variables|/Script/Engine.SceneComponent|GetRelativeLocation (Variables|Default|GetDoor_L)))
  (Variables|Default|SetInitialLoc_R (Variables|/Script/Engine.SceneComponent|GetRelativeLocation (Variables|Default|GetDoor_R))))