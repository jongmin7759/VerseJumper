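; BP_MainMenuActor runs the main menu scene, from the initial press-any-key screen to the camera transition that follows it.
; On BeginPlay it sets the verse state to AlphaVerse, shows the WBP_MainMenu widget with a mouse cursor and fades in the theme music.
; The widget's press-any-key callback switches the verse to TrashVerse, eases the view to a second camera and plays a glitch sound.
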(event Custom|PressAnyKeyEvent_Event
  (Class|VerseStateSubsystem|SetNewState (Subsystems|GetVerseStateSubsystem) (GameplayTags|MakeLiteralGameplayTag "(TagName=\"VerseState.TrashVerse\")"))
  (Game|Player|SetViewTargetwithBlend (Game|GetPlayerController 0) (Variables|Default|GetNewCameraRef) 2.0 "VTBlend_EaseInOut" 5.0 false)
  (Audio|PlaySound2D "/Game/Asset/SCI-FI_UI_SFX_PACK/Glitches/Glitch_Cue.Glitch_Cue" 1.0 1.0 0.0 0 0))

(event EventBeginPlay
  (Utilities|FlowControl|Sequence
    (:then_0
      (Class|VerseStateSubsystem|SetNewState (Subsystems|GetVerseStateSubsystem) (GameplayTags|MakeLiteralGameplayTag "(TagName=\"VerseState.AlphaVerse\")")))
    (:then_1
      (bind _returnvalue (UserInterface|CreateWidget "/Game/Blueprint/MainMenu/WBP_MainMenu.WBP_MainMenu_C" (Game|GetPlayerController 0)))
      (bind _output_get (Variables|Default|SetMainMenu _returnvalue))
      (UserInterface|Viewport|AddtoViewport _output_get 0)
      (Widget|SetFocus (Variables|Default|GetMainMenu))
      (Variables|/Script/Engine.PlayerController|SetbShowMouseCursor (Game|GetPlayerController 0) true)
      (Audio|Components|Audio|FadeIn (Variables|Default|GetMainTheme_Cue) 5.0 1.0 0.0 "Linear" :!class /Script/Engine.AudioComponent))
    (:then_2
      (EventDispatchers|AssignPressAnyKeyEvent (Variables|Default|GetMainMenu) (delegate Custom|PressAnyKeyEvent_Event)))))

(fn ConstructionScript)