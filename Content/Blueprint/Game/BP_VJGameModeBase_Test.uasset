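; Test variant of the VJ game mode that starts the player at a dedicated test spawn with cheats on.
; ChoosePlayerStart is overridden to look up the player start named "Test".
; On BeginPlay, after the parent logic runs, it casts the first player pawn to BP_VJPlayerCharacter and enables cheats on it.
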(event EventBeginPlay
  (|CallParentFunction)
  (bind _asbp_vjplayer_character (Utilities|Casting|CastToBP_VJPlayerCharacter (Game|Player|GetPlayerPawn 0)))
  (Default|EnableCheat _asbp_vjplayer_character))

(event EventTick
  (params (DeltaSeconds :type Float%20%28single-precision%29))
  (|CallParentFunction DeltaSeconds) ; 지금 이 노드는 비활성 상태입니다. \n핀을 끌어서 다른 노드를 연결하면 활성화됩니다.
)

(fn ConstructionScript
  (|CallParentFunction))

(fn ChoosePlayerStart
  (params (Player :type Controller%20Object%20Reference))
  (return (Class|GameModeBase|FindPlayerStart Player "Test")))