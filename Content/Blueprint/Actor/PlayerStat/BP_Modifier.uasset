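; BP_Modifier is a one-time interactable pickup that grants the modifier to the player character.
; On interaction it plays a level sequence while notifying the player controller, flags the character as having the modifier, saves itself and hides.
; When the sequence finishes, the controller is notified and the actor is destroyed.
; The LifeCycleSave component also destroys it on load if it was already collected.
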(event OnInteractSuccess(InteractionComponent)
  (params (InstigatorController :type Player%20Controller%20Object%20Reference))
  (Utilities|FlowControl|Sequence
    (:then_0
      (CallFunction|PlaySequence))
    (:then_1
      (bind _asvjplayer_character (Utilities|Casting|CastToVJPlayerCharacter (Pawn|GetControlledPawn InstigatorController)))
      (Class|VJPlayerCharacter|SetHasModifier _asvjplayer_character true)
      (Variables|Default|SetAlreadyGet true)
      (Class|LifeCycleSaveComponent|SaveOwnerActor (Variables|Default|GetLifeCycleSave))
      (Rendering|SetActorHiddenInGame true))))

(event OnLoaded(LifeCycleSave)
  (if (Variables|Default|GetAlreadyGet)
    (Actor|DestroyActor)))

(event Custom|EndSequnce
  (Class|VJPlayerController|HandleSequneceStopped (Variables|Default|GetAs%20VJPlayer%20Controller))
  (Actor|DestroyActor))

(fn ConstructionScript
  (|CallParentFunction))

(fn PlaySequence
  (bind _sequence (Variables|Sequence|GetSequence))
  (bind _sequenceplayer (Variables|/Script/LevelSequence.LevelSequenceActor|GetSequencePlayer _sequence))
  (bind _asvjplayer_controller (Utilities|Casting|CastToVJPlayerController (Game|GetPlayerController 0)))
  (bind _output_get (Variables|Default|SetAs%20VJPlayer%20Controller _asvjplayer_controller))
  (Class|VJPlayerController|HandleSequnecePlaying _output_get)
  (Sequencer|Player|Play _sequenceplayer :!class /Script/MovieScene.MovieSceneSequencePlayer)
  (EventDispatchers|BindEventtoOnFinished _sequenceplayer (EventDispatchers|CreateEvent :!event Custom|EndSequnce)))