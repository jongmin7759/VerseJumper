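; Card key pickup that the player collects by interacting with it, with state persisted across saves.
; Tick bobs it along its up vector on a time-based sine, though the degree-based Sind receives a radian-scaled angle, so Frequency is not in hertz.
; A successful interaction plays a sound, sets the card key flag on the VJPlayerCharacter, saves through LifeCycleSave and destroys the actor.
; On load, an already collected key destroys itself.
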(event OnInteractSuccess(InteractionComponent)
  (params (InstigatorController :type Player%20Controller%20Object%20Reference))
  (Audio|PlaySound2D "/Game/Asset/SCI-FI_UI_SFX_PACK/Tone1/Major/GetCollectible_Cue.GetCollectible_Cue" 1.0 1.0 0.0 0 0)
  (bind _asvjplayer_character (Utilities|Casting|CastToVJPlayerCharacter (Pawn|GetControlledPawn InstigatorController)))
  (Class|VJPlayerCharacter|SetHasCardKey _asvjplayer_character true)
  (Variables|Default|SetAlreadyGet true)
  (Class|LifeCycleSaveComponent|SaveOwnerActor (Variables|Default|GetLifeCycleSave))
  (Actor|DestroyActor))

(event OnLoaded(LifeCycleSave)
  (if (Variables|Default|GetAlreadyGet)
    (Actor|DestroyActor)))

(event EventTick
  (params (DeltaSeconds :type Float%20%28single-precision%29))
  (Transformation|SetActorLocation (+ (Variables|Default|GetOriginalLoc) (* (Transformation|GetActorUpVector) (Math|Trig|Sin(Degrees) (* (Utilities|Time|GetTimeSeconds) (Math|Trig|GetPI) 2.0 (Variables|Default|GetFrequency))) (Variables|Default|GetAmplitude))) false false))

(event EventBeginPlay
  (Variables|Default|SetOriginalLoc (Transformation|GetActorLocation)))

(fn ConstructionScript
  (|CallParentFunction))