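; One-time interactable pickup that grants the player the TrashVerse state and unlocks the Story_dial achievement.
; On successful interaction it plays an optional sequence, adds the state through the pawn's PlayerVerseStateComponent, saves itself and hides.
; The player controller is notified when the sequence plays and stops, and EndSequence destroys the actor.
; The saved AlreadyGet flag makes the actor destroy itself on load once collected.
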(event OnInteractSuccess(InteractionComponent)
  (params (InstigatorController :type Player%20Controller%20Object%20Reference))
  (CallFunction|PlaySequence)
  (bind _asvjplayer_character (Utilities|Casting|CastToVJPlayerCharacter (Pawn|GetControlledPawn InstigatorController)))
  (Class|PlayerVerseStateComponent|AddAvailableState (Variables|/Script/VerseJumper.VJPlayerCharacter|GetPlayerVerseStateComponent _asvjplayer_character) "(TagName=\"VerseState.TrashVerse\")")
  (Variables|Default|SetAlreadyGet true)
  (Class|LifeCycleSaveComponent|SaveOwnerActor (Variables|Default|GetLifeCycleSave) false)
  (Rendering|SetActorHiddenInGame true)
  (bind _asvjgame_mode_base (Utilities|Casting|CastToVJGameModeBase (Game|GetGameMode)))
  (Class|VJGameModeBase|UnlockAchievement _asvjgame_mode_base "Story_dial"))

(event OnLoaded(LifeCycleSave)
  (if (Variables|Default|GetAlreadyGet)
    (Actor|DestroyActor)))

(event Custom|EndSequence
  (Class|VJPlayerController|HandleSequneceStopped (Variables|Default|GetAs%20VJPlayer%20Controller))
  (Actor|DestroyActor))

(fn ConstructionScript
  (|CallParentFunction))

(fn PlaySequence
  (bind _sequence (Variables|Default|GetSequence))
  (bind _sequenceplayer (Variables|/Script/LevelSequence.LevelSequenceActor|GetSequencePlayer _sequence))
  (Utilities|IsValid (Variables|Default|GetSequence)
    (:Is%20Valid
      (bind _asvjplayer_controller (Utilities|Casting|CastToVJPlayerController (Game|GetPlayerController 0)))
      (bind _output_get (Variables|Default|SetAs%20VJPlayer%20Controller _asvjplayer_controller))
      (Class|VJPlayerController|HandleSequnecePlaying _output_get)
      (Sequencer|Player|Play _sequenceplayer :!class /Script/MovieScene.MovieSceneSequencePlayer)
      (EventDispatchers|BindEventtoOnFinished _sequenceplayer (EventDispatchers|CreateEvent :!event Custom|EndSequence)))))