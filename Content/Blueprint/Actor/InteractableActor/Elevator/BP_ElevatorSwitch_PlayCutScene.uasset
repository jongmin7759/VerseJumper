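; Elevator switch variant that plays a cutscene sequence when used, as long as it is not flagged as already used.
; BeginPlay caches the VJPlayerController from player 0.
; UseSwitch runs the parent logic, then, if AlreadyUsed is false, notifies the controller, plays the Sequence's player and binds its OnFinished event.
; An EndSequence event tells the controller the sequence has stopped.
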(event Custom|EndSequence
  (Class|VJPlayerController|HandleSequneceStopped (Variables|Default|GetVJPlayer%20Controller)))

(event EventBeginPlay
  (|CallParentFunction)
  (bind _asvjplayer_controller (Utilities|Casting|CastToVJPlayerController (Game|GetPlayerController 0)))
  (Variables|Default|SetVJPlayer%20Controller _asvjplayer_controller))

(fn ConstructionScript
  (|CallParentFunction))

(fn UseSwitch
  (bind _sequence (Variables|Sequence|GetSequence))
  (bind _sequenceplayer (Variables|/Script/LevelSequence.LevelSequenceActor|GetSequencePlayer _sequence))
  (|CallParentFunction)
  (if (not (Variables|Default|GetAlreadyUsed))
    (Class|VJPlayerController|HandleSequnecePlaying (Variables|Default|GetVJPlayer%20Controller))
    (Sequencer|Player|Play _sequenceplayer :!class /Script/MovieScene.MovieSceneSequencePlayer)
    (EventDispatchers|BindEventtoOnFinished _sequenceplayer (EventDispatchers|CreateEvent :!event Custom|EndSequence))))