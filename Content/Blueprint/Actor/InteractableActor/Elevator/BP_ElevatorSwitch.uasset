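; Interactable elevator switch that starts or stops the MoverComponents of its linked MoverActor list, with sounds for interaction attempts and movement.
; A successful interaction toggles every mover not flagged fixed and saves the switch through LifeCycleSave.
; Loading a used switch calls FixLocation on moving platform movers with their target location, then replays the toggle, guarded against repeats.
; Highlight events mirror custom depth and stencil color onto the linked actors' meshes.
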(event OnInteractSuccess(InteractionComponent)
  (params (InstigatorController :type Player%20Controller%20Object%20Reference))
  (CallFunction|UseSwitch)
  (Variables|Default|SetAlreadyUsed true)
  (Class|LifeCycleSaveComponent|SaveOwnerActor (Variables|Default|GetLifeCycleSave))
  (Variables|Default|SetAlreadyLoaded true))

(event OnLoaded(LifeCycleSave)
  (if (not (Variables|Default|GetAlreadyLoaded))
    (if (Variables|Default|GetAlreadyUsed)
      (CallFunction|FixLocation)
      (CallFunction|UseSwitch)
      (Variables|Default|SetAlreadyLoaded true))))

(event OnTryInteract(InteractionComponent)
  (Audio|SpawnSoundatLocation (Variables|DeviceProperties|GetDeviceSound) (Transformation|GetActorLocation) "0, 0, 0" 1.0 1.0 0.0 0 0))

(event EventOnHighlight
  (for _array_element (Variables|DeviceProperties|GetMoverActor)
    (Utilities|IsValid (Actor|GetComponentbyClass _array_element "/Script/Engine.StaticMeshComponent")
      (:Is%20Valid
        (Rendering|SetRenderCustomDepth (Actor|GetComponentbyClass _array_element "/Script/Engine.StaticMeshComponent") true)))))

(event EventOnUnHighlight
  (for _array_element (Variables|DeviceProperties|GetMoverActor)
    (Utilities|IsValid (Actor|GetComponentbyClass _array_element "/Script/Engine.StaticMeshComponent")
      (:Is%20Valid
        (Rendering|SetRenderCustomDepth (Actor|GetComponentbyClass _array_element "/Script/Engine.StaticMeshComponent") false)))))

(event EventOnHighlightColorChanged
  (params (Value :type Integer))
  (Variables|Default|SetValue Value)
  (for _array_element (Variables|DeviceProperties|GetMoverActor)
    (Utilities|IsValid (Actor|GetComponentbyClass _array_element "/Script/Engine.StaticMeshComponent")
      (:Is%20Valid
        (Rendering|SetCustomDepthStencilValue (Actor|GetComponentbyClass _array_element "/Script/Engine.StaticMeshComponent") (Variables|Default|GetValue))))))

(fn ConstructionScript
  (|CallParentFunction))

(fn UseSwitch
  (for _array_element (Variables|DeviceProperties|GetMoverActor)
    (Utilities|IsValid (Actor|GetComponentbyClass _array_element "/Script/VerseJumper.MoverComponent")
      (:Is%20Valid
        (if (not (Class|MoverComponent|IsFixed (Actor|GetComponentbyClass _array_element "/Script/VerseJumper.MoverComponent")))
          (Audio|SpawnSoundatLocation (Variables|DeviceProperties|GetMoveActorSound) (Transformation|GetActorLocation _array_element) "0, 0, 0" 1.0 1.0 0.0 "/Game/Audio/Attenuation/SA_Default.SA_Default" 0)
          (if (Class|MoverComponent|IsActivated (Actor|GetComponentbyClass _array_element "/Script/VerseJumper.MoverComponent"))
            (Class|MoverComponent|StopMoving (Actor|GetComponentbyClass _array_element "/Script/VerseJumper.MoverComponent"))
            (else
              (Class|MoverComponent|StartMoving (Actor|GetComponentbyClass _array_element "/Script/VerseJumper.MoverComponent")))))))))

(fn FixLocation
  (for _array_element (Variables|DeviceProperties|GetMoverActor)
    (Utilities|IsValid (Actor|GetComponentbyClass _array_element "/Script/VerseJumper.MoverComponent")
      (:Is%20Valid
        (bind _asbp_moving_platform_base (Utilities|Casting|CastToBP_MovingPlatformBase _array_element))
        (Class|MoverComponent|FixLocation (Actor|GetComponentbyClass _array_element "/Script/VerseJumper.MoverComponent") (Math|Transform|TransformLocation (Transformation|GetActorTransform _asbp_moving_platform_base) (Variables|/Game/Blueprint/Actor/PlatformActor/MovingPlatform/BP_MovingPlatformBase.BP_MovingPlatformBase_C|GetTargetLocation _asbp_moving_platform_base)))))))