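; Interactable start-scene device that opens a linked door actor once.
; A successful interaction plays sparks and sounds, turns a material slot to black glass, and runs a Timeline lerping the door to TargetLocation.
; When the Timeline finishes, it disables interaction and saves through LifeCycleSave, which restores the opened door and interaction state on load.
; Failed interactions reuse the same sound and spark functions without moving the door.
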(event OnInteractSuccess(InteractionComponent)
  (params (InstigatorController :type Player%20Controller%20Object%20Reference))
  (Utilities|FlowControl|DoOnce false
    (:Completed
      (Utilities|FlowControl|Sequence
        (:then_0
          (CallFunction|PlaySound)
          (CallFunction|SpawnParticle)
          (Rendering|Material|SetMaterial (Variables|Default|GetStaticMesh) 2 "/Game/Asset/SciFi_BioLaboratory/Materials/Glass/MI_Black_Glass.MI_Black_Glass"))
        (:then_1
          (Utilities|IsValid (Variables|Door|GetDoorActor)
            (:Is%20Valid
              (bind _alpha (Timeline|Timeline Play)
                (:Update
                  (Transformation|SetActorLocation (Variables|Door|GetDoorActor) (Math|Vector|Lerp(Vector) (Variables|Default|GetStartLocation) (Variables|Door|GetTargetLocation) _alpha) false false))
                (:Finished
                  (Variables|Default|SetbIsUsed true)
                  (Class|LifeCycleSaveComponent|SaveOwnerActor (Variables|Default|GetLifeCycleSave) false)
                  (Variables|/Script/VerseJumper.InteractionComponent|SetbCanInteract (Variables|Default|GetInteractionComponent) false))))))))))

(event OnLoaded(LifeCycleSave)
  (Variables|/Script/VerseJumper.InteractionComponent|SetbCanInteract (Variables|Default|GetInteractionComponent) (not (Variables|Default|GetbIsUsed)))
  (if (Variables|Default|GetbIsUsed)
    (Transformation|SetActorLocation (Variables|Door|GetDoorActor) (Variables|Door|GetTargetLocation) false false)))

(event OnInteractFailed(InteractionComponent)
  (params (InstigatorController :type Player%20Controller%20Object%20Reference))
  (CallFunction|PlaySound)
  (CallFunction|SpawnParticle))

(event EventBeginPlay
  (bind _dooractor (Variables|Door|GetDoorActor))
  (|CallParentFunction)
  (Utilities|IsValid _dooractor
    (:Is%20Valid
      (Variables|Default|SetStartLocation (Transformation|GetActorLocation _dooractor)))))

(fn ConstructionScript
  (|CallParentFunction))

(fn PlaySound
  (Utilities|FlowControl|Sequence
    (:then_0
      (Audio|PlaySoundatLocation "/Game/Asset/SCI-FI_UI_SFX_PACK/Glitches/Glitch_Single_Cue.Glitch_Single_Cue" (Transformation|GetActorLocation) "0, 0, 0" 1.0 1.0 0.0 "/Game/Audio/Attenuation/SA_Default.SA_Default" 0 0 0)
      (Audio|PlaySoundatLocation "/Game/Asset/SFX/ElectricSpark_Cue.ElectricSpark_Cue" (Transformation|GetActorLocation) "0, 0, 0" 0.5 1.0 0.0 "/Game/Audio/Attenuation/SA_Default.SA_Default" 0 0 0))
    (:then_1
      (if (not (Variables|Default|GetbIsUsed))
        (Audio|PlaySoundatLocation "/Game/Asset/SCI-FI_UI_SFX_PACK/Click_Combos/UseDevice_Cue.UseDevice_Cue" (Transformation|GetActorLocation) "0, 0, 0" 1.0 1.0 0.0 0 0 0 0)
        (Audio|PlaySoundatLocation "/Game/Asset/SFX/OpeningRollDoor_Cue.OpeningRollDoor_Cue" (Variables|Default|GetStartLocation) "0, 0, 0" 1.0 1.0 0.0 "/Game/Audio/Attenuation/SA_Default.SA_Default" 0 0 0)))))

(fn SpawnParticle
  (Effects|SpawnEmitterAttached "/Game/Asset/Realistic_Starter_VFX_Pack_Vol2/Particles/Sparks/P_Sparks_C_Once.P_Sparks_C_Once" (Variables|Default|GetSpark_1) "None")
  (Effects|SpawnEmitterAttached "/Game/Asset/Realistic_Starter_VFX_Pack_Vol2/Particles/Sparks/P_Sparks_C_Once.P_Sparks_C_Once" (Variables|Default|GetSpark_2) "None"))