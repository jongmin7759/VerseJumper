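; BP_DoorSwitch is a one-time interactable switch that opens a linked Door, usable only when the player carries a key card.
; On each interaction attempt it sets CanInteract from HasCardKey and the used state.
; A successful use opens the Door, disables further interaction and saves through LifeCycleSave, which reopens the Door on load.
; Highlight events forward custom depth and stencil color to the Door's static mesh.
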(event OnInteractSuccess(InteractionComponent)
  (params (InstigatorController :type Player%20Controller%20Object%20Reference))
  (Default|Open (Variables|Default|GetDoor) false)
  (Variables|Default|SetbIsUsed true)
  (Class|LifeCycleSaveComponent|SaveOwnerActor (Variables|Default|GetLifeCycleSave))
  (Variables|/Script/VerseJumper.InteractionComponent|SetbCanInteract (Variables|Default|GetInteractionComponent) false))

(event OnLoaded(LifeCycleSave)
  (if (Variables|Default|GetbIsUsed)
    (Default|Open (Variables|Default|GetDoor) true)
    (Variables|/Script/VerseJumper.InteractionComponent|SetbCanInteract (Variables|Default|GetInteractionComponent) false)))

(event OnTryInteract(InteractionComponent)
  (if (Variables|Default|GetbIsUsed)
    (Variables|/Script/VerseJumper.InteractionComponent|SetbCanInteract (Variables|Default|GetInteractionComponent) false)
    (else
      (bind _asvjplayer_character (Utilities|Casting|CastToVJPlayerCharacter (Game|Player|GetPlayerPawn 0)))
      (Variables|/Script/VerseJumper.InteractionComponent|SetbCanInteract (Variables|Default|GetInteractionComponent) (Variables|/Script/VerseJumper.VJPlayerCharacter|GetbHasCardKey _asvjplayer_character)))))

(event EventOnHighlight
  (bind _door (Variables|Default|GetDoor))
  (bind _returnvalue (Actor|GetComponentbyClass _door "/Script/Engine.StaticMeshComponent"))
  (Utilities|IsValid _returnvalue
    (:Is%20Valid
      (Rendering|SetRenderCustomDepth _returnvalue true))))

(event EventOnUnHighlight
  (bind _door (Variables|Default|GetDoor))
  (bind _returnvalue (Actor|GetComponentbyClass _door "/Script/Engine.StaticMeshComponent"))
  (Utilities|IsValid _returnvalue
    (:Is%20Valid
      (Rendering|SetRenderCustomDepth _returnvalue false))))

(event EventOnHighlightColorChanged
  (params (Value :type Integer))
  (bind _door (Variables|Default|GetDoor))
  (bind _returnvalue (Actor|GetComponentbyClass _door "/Script/Engine.StaticMeshComponent"))
  (Variables|Default|SetValue Value)
  (Utilities|IsValid _returnvalue
    (:Is%20Valid
      (Rendering|SetCustomDepthStencilValue _returnvalue (Variables|Default|GetValue)))))

(fn ConstructionScript
  (|CallParentFunction))