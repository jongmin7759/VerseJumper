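; Test collectible actor that the player picks up through its interaction component.
; On a successful interaction it registers its CollectibleID with the VJPlayerCharacter's CollectibleTracker, sets AlreadyGet, saves itself through the LifeCycleSave component and destroys itself.
; When LifeCycleSave finishes loading, the actor destroys itself if AlreadyGet is set, so collected items stay gone.
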(event OnInteractSuccess(InteractionComponent)
  (params (InstigatorController :type Player%20Controller%20Object%20Reference))
  (bind _asvjplayer_character (Utilities|Casting|CastToVJPlayerCharacter (Pawn|GetControlledPawn InstigatorController)))
  (Class|CollectibleTrackerComponent|RegisterCollectible (Variables|/Script/VerseJumper.VJPlayerCharacter|GetCollectibleTracker _asvjplayer_character) (Variables|Default|GetCollectible%20ID))
  (Variables|Default|SetAlreadyGet true)
  (Class|LifeCycleSaveComponent|SaveOwnerActor (Variables|Default|GetLifeCycleSave_0))
  (Actor|DestroyActor))

(event OnLoaded(LifeCycleSave_0)
  (if (Variables|Default|GetAlreadyGet)
    (Actor|DestroyActor)))

(fn ConstructionScript
  (|CallParentFunction))