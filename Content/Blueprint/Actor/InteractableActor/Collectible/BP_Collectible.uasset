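; BP_Collectible is an interactable collectible actor that the player picks up once.
; On a successful interaction it registers its CollectibleID with the VJPlayerCharacter's CollectibleTracker, marks itself as obtained, saves through LifeCycleSave and destroys itself.
; When LifeCycleSave finishes loading, it destroys itself again if already obtained, so collected items stay gone.
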(event OnInteractSuccess(InteractionComponent)
  (params (InstigatorController :type Player%20Controller%20Object%20Reference))
  (bind _asvjplayer_character (Utilities|Casting|CastToVJPlayerCharacter (Pawn|GetControlledPawn InstigatorController)))
  (Class|CollectibleTrackerComponent|RegisterCollectible (Variables|/Script/VerseJumper.VJPlayerCharacter|GetCollectibleTracker _asvjplayer_character) (Variables|CollectibleProperties|GetCollectible%20ID))
  (Variables|CollectibleProperties|SetAlreadyGet true)
  (Class|LifeCycleSaveComponent|SaveOwnerActor (Variables|Default|GetLifeCycleSave))
  (Actor|DestroyActor))

(event OnLoaded(LifeCycleSave)
  (if (Variables|CollectibleProperties|GetAlreadyGet)
    (Actor|DestroyActor)))

(fn ConstructionScript
  (|CallParentFunction))