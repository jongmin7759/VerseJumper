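; BP_VerseJumpStand_OneVerse is an interactable stand that switches the game to one set verse state.
; When its InteractionComponent reports a successful interaction, it passes NewState to the VerseStateSubsystem and plays a sound at the actor's location.
; All logic lives in that one event, with no active BeginPlay, overlap or Tick handling.
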(event OnInteractSuccess(InteractionComponent)
  ;[0.15 0.15 0.15 0.5] 실제 상호작용 구현
  (Class|VerseStateSubsystem|SetNewState (Subsystems|GetVerseStateSubsystem) (Variables|Default|GetNew%20State))
  (Audio|PlaySoundatLocation "/Game/Audio/SFX/Modifier/ChangeTargetState.ChangeTargetState" (Transformation|GetActorLocation) "0, 0, 0" 1.0 1.0 0.0 0 0 0 0))

(event EventBeginPlay
  (|CallParentFunction) ; This node is disabled and will not be called.\nDrag off pins to build functionality.
)

(event Collision|EventActorBeginOverlap
  (params (OtherActor :type Actor%20Object%20Reference))
  (|CallParentFunction OtherActor) ; This node is disabled and will not be called.\nDrag off pins to build functionality.
)

(event EventTick
  (params (DeltaSeconds :type Float%20%28single-precision%29))
  (|CallParentFunction DeltaSeconds) ; This node is disabled and will not be called.\nDrag off pins to build functionality.
)

(fn ConstructionScript
  (|CallParentFunction))