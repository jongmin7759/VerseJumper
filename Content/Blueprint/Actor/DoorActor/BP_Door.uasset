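; BP_Door is a double door actor that slides its left and right meshes open when Open is called.
; BeginPlay caches both meshes' relative locations as start points.
; Open fires OpenDoorEvent, whose OpenDoor timeline lerps each mesh to its target, with no close logic.
; UpdateTargetLocation duplicates UpdateStartLocation, writing the start variables, so the target variables are never assigned in these graphs.
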(event Custom|OpenDoorEvent
  (bind _alpha (Timeline|OpenDoor Play)
    (:Update
      (Transformation|SetRelativeLocation (Variables|Default|GetSM_Door_Left) (Math|Vector|Lerp(Vector) (Variables|Default|GetLeftDoorStart) (Variables|Default|GetLeftDoorTarget) _alpha) false false)
      (Transformation|SetRelativeLocation (Variables|Default|GetSM_Door_Right) (Math|Vector|Lerp(Vector) (Variables|Default|GetRightDoorStart) (Variables|Default|GetRightDoorTarget) _alpha) false false))))

(event EventBeginPlay
  (CallFunction|UpdateStartLocation))

(fn ConstructionScript)

(fn Open
  (CallFunction|OpenDoorEvent))

(fn UpdateStartLocation
  (Variables|Default|SetLeftDoorStart (Variables|/Script/Engine.SceneComponent|GetRelativeLocation (Variables|Default|GetSM_Door_Left)))
  (Variables|Default|SetRightDoorStart (Variables|/Script/Engine.SceneComponent|GetRelativeLocation (Variables|Default|GetSM_Door_Right))))

(fn UpdateTargetLocation
  (Variables|Default|SetLeftDoorStart (Variables|/Script/Engine.SceneComponent|GetRelativeLocation (Variables|Default|GetSM_Door_Left)))
  (Variables|Default|SetRightDoorStart (Variables|/Script/Engine.SceneComponent|GetRelativeLocation (Variables|Default|GetSM_Door_Right))))