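; Egyptian pillar variant of a moving platform, built on a parent platform Blueprint.
; On BeginPlay, when flagged for sequence use, it swaps in sequence-specific moving and arrival sound cues.
; When its Mover component finishes moving, it triggers a dust ring Niagara effect and a short camera shake on the first player's camera.
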(event OnMoveEnded(Mover)
  (Components|Activation|Activate (Variables|Default|GetNS_DustRing) false)
  (CameraShakes|StartCameraShake (Variables|/Script/Engine.PlayerController|GetPlayerCameraManager (Game|GetPlayerController 0)) "/Game/Blueprint/CameraShake/BP_CameraShake_Short.BP_CameraShake_Short_C" 1.0 "CameraLocal" "0, 0, 0"))

(event EventBeginPlay
  (|CallParentFunction)
  (if (Variables|Sequence|GetForSequence)
    (Variables|Default|SetMovingSound "/Game/Asset/SFX/MovingPillar_Sequence_Cue.MovingPillar_Sequence_Cue")
    (Variables|Default|SetArriveSound "/Game/Asset/SFX/Stomp_Sequence_Cue.Stomp_Sequence_Cue")))

(fn ConstructionScript
  (|CallParentFunction))