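; BP_MovingPlatformBase is a base moving platform actor that travels toward a configurable relative TargetLocation with movement audio.
; BeginPlay passes the target to the Mover component, whose start and end events fade the AudioComponent in and out and print debug strings.
; MovingSound is async-loaded on a move start when no sound is set, then assigned and faded in.
; A debug box preview of the target in the construction script is disconnected.
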(event OnMoveStarted(Mover)
  (bind _audiocomponent (Variables|Default|GetAudioComponent))
  (Development|PrintString "Move Start")
  (if (Utilities|IsValid (Variables|/Script/Engine.AudioComponent|GetSound (Variables|Default|GetAudioComponent)))
    _
    (else
      (bind _object (Utilities|AsyncLoadAsset (Variables|Default|GetMovingSound))
        (:Completed
          (bind _assound_base (Utilities|Casting|CastToSoundBase _object))
          (Audio|Components|Audio|SetSound _audiocomponent _assound_base)))))
  (Audio|Components|Audio|FadeIn _audiocomponent 0.5 1.0 0.0 "Linear" :!class /Script/Engine.AudioComponent))

(event OnMoveEnded(Mover)
  (Audio|Components|Audio|FadeOut (Variables|Default|GetAudioComponent) 0.5 0.0 "Linear" :!class /Script/Engine.AudioComponent)
  (Development|PrintString "Hello"))

(event EventBeginPlay
  (Class|MoverComponent|SetRelativeTargetLocation (Variables|Default|GetMover) (Variables|Default|GetTargetLocation)))

(fn ConstructionScript)