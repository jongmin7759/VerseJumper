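; Test actor for movement, built around a Mover that receives a zero target location on BeginPlay.
; The construction script caches the original location, and EndPlay records the game time.
; A disconnected, never-run Timeline graph would loop a vertical offset scaled by TargetZ, using that end time to resume in phase over a two-second cycle.
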(event EventBeginPlay
  (Class|MoverComponent|SetTargetLocation (Variables|Default|GetMover) "0, 0, 0"))

(event EventEndPlay
  (params (EndPlayReason :type EEndPlayReason%20Enum :default "Destroyed"))
  (Variables|Default|SetEndTime (Utilities|Time|GetGameTimeinSeconds)))

(fn ConstructionScript
  (Variables|Default|SetOriginalLocation (Transformation|GetActorLocation)))